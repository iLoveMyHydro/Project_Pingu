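; BP_Enemy is an enemy actor that loses health when damaged and destroys itself when health reaches zero or below.
; A GetDamage event calls an ApplyDamage wrapper, which routes the hit to itself through Unreal's built-in damage system.
; The AnyDamage event then passes the truncated damage to the GetDamage function, which subtracts it from Health and handles destruction.
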(event Custom|Get%20Damage
  (params (Damage :type Integer))
  ;[1 1 1] Damage
  (CallFunction|ApplyDamage Damage))

(event Game|Damage|EventAnyDamage
  (params (Damage :type Float%20%28single-precision%29) (DamageType :type Damage%20Type%20Object%20Reference) (InstigatedBy :type Controller%20Object%20Reference) (DamageCauser :type Actor%20Object%20Reference))
  ;[1 1 1] Damage
  (CallFunction|GetDamage (Math|Float|Truncate Damage)))

(fn ConstructionScript)

(fn ApplyDamage
  (params (Damage :type Integer))
  (Game|Damage|ApplyDamage self (Math|Conversions|ToFloat(Integer) Damage) 0 0 "/Script/Engine.DamageType"))

(fn GetDamage
  (params (Damage :type Integer))
  (bind _output_get (Variables|Default|SetHealth (Math|Float|Truncate (- (Variables|Default|GetHealth) Damage))))
  (if (<= _output_get 0)
    (Actor|DestroyActor)))