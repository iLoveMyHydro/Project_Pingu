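; Enemy AI controller that starts the BT_Enemy behavior tree and passes sight perception results to its Blackboard.
; HandleSightSense filters perception updates to sight, then sets TargetActor to the player, or to none when the stimulus is not successfully sensed.
; CanSeePlayer depends only on whether the updated actor is the player, so it stays true on sight loss.
; Each sight update prints a green or red debug message.
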(event OnTargetPerceptionUpdated(AIPerception)
  (params (Actor :type Actor%20Object%20Reference) (Stimulus :type AI%20Stimulus%20Structure))
  (CallFunction|HandleSightSense Actor Stimulus))

(event EventBeginPlay
  (AI|RunBehaviorTree "/Game/Blueprint/AI/BT_Enemy.BT_Enemy"))

(fn ConstructionScript)

(fn HandleSightSense
  (params (Actor :type Actor%20Object%20Reference) (Stimulus :type AI%20Stimulus%20Structure))
  (bind _returnvalue (Class|AIPerceptionSystem|GetSenseClassforStimulus Stimulus))
  (if (== _returnvalue "/Script/AIModule.AISense_Sight")
    (if (== Actor (Game|GetPlayerCharacter 0))
      (AI|Components|Blackboard|SetValueasObject (Variables|Default|GetBlackboard) (Utilities|Name|MakeLiteralName "TargetActor") (Utilities|SelectObject (Game|GetPlayerCharacter 0) 0 (.bsuccessfullysensed Stimulus)))
      (AI|Components|Blackboard|SetValueasBool (Variables|Default|GetBlackboard) (Utilities|Name|MakeLiteralName "CanSeePlayer") true)
      (Development|PrintString "CanSeePlayer" true true "(R=0.000000,G=1.000000,B=0.000000,A=1.000000)")
      (else
        (AI|Components|Blackboard|SetValueasObject (Variables|Default|GetBlackboard) (Utilities|Name|MakeLiteralName "TargetActor") (Utilities|SelectObject (Game|GetPlayerCharacter 0) 0 (.bsuccessfullysensed Stimulus)))
        (AI|Components|Blackboard|SetValueasBool (Variables|Default|GetBlackboard) (Utilities|Name|MakeLiteralName "CanSeePlayer") false)
        (Development|PrintString "CanSeePlayer" true true "(R=1.000000,G=0.000000,B=0.000000,A=1.000000)")
        (return)))
    (else
      (return))))