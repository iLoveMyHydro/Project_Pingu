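; Player character Blueprint that handles input setup, life, pausing and a slap attack.
; BeginPlay adds the Enhanced Input mapping, initializes BPPlayerMovement and creates the life HUD, which refreshes on life changes.
; Actor overlaps track the current enemy for slap damage, while life below zero triggers mesh physics and a Game Over widget.
; A pause menu toggles game pause and input mode, and raw keys adjust life or destroy the actor.
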(event Custom|Update%20Life
  (params (Amount :type Integer) (Max%20Life :type Boolean))
  ;[0.3532 1 0.2572] Life System
  (CallFunction|UpdateLife Amount Max%20Life))

(event Input|EnhancedActionEvents|EnhancedInputActionIA_Slap
  (params (ActionValue :type Boolean) (ElapsedSeconds :type Float%20%28double-precision%29) (TriggeredSeconds :type Float%20%28double-precision%29) (InputAction :type Input%20Action%20Object%20Reference :default "/Game/Input/Actions/IA_Slap.IA_Slap"))
  ;[0.3176 0.3319 1] Slap
  (:Started
    (CallFunction|OnSlap))
  (:Completed
    (Variables|Default|SetIsAttacking false)
    (Development|SetHiddeninGame (Variables|Default|GetHitbox) true false)))

(event Input|EnhancedActionEvents|EnhancedInputActionIA_Pause
  (params (ActionValue :type Boolean) (ElapsedSeconds :type Float%20%28double-precision%29) (TriggeredSeconds :type Float%20%28double-precision%29) (InputAction :type Input%20Action%20Object%20Reference :default "/Game/Input/Actions/IA_Pause.IA_Pause"))
  ;[1 0.8395 0.3297] Pause Menu
  (CallFunction|PauseMenu))

(event EventBeginPlay
  ;[1 0.2226 0.9329 1 34] Init Movement and Init Life System
  (CallFunction|SetInputMapping)
  (Default|InitMovement (Variables|Default|GetBP_PlayerMovement) self)
  (bind _returnvalue (UserInterface|CreateWidget "/Game/HUD/WBP_Hud_Lifesystem.WBP_Hud_Lifesystem_C"))
  (bind _output_get (Variables|Default|SetHudLifeRef _returnvalue))
  (UserInterface|Viewport|AddtoViewport _returnvalue 0))

(event Collision|EventActorBeginOverlap
  (params (OtherActor :type Actor%20Object%20Reference))
  ;[0.3176 0.3319 1] Slap
  (bind _asbp_enemy_ (Utilities|Casting|CastToBP_Enemy_ OtherActor))
  (Variables|Default|SetCurrentEnemy _asbp_enemy_)
  (Variables|Default|SetIsColliding true))

(event Collision|EventActorEndOverlap
  (params (OtherActor :type Actor%20Object%20Reference))
  ;[0.3176 0.3319 1] Slap
  (Utilities|Casting|CastToBP_Enemy_ OtherActor)
  (Variables|Default|SetCurrentEnemy 0)
  (Variables|Default|SetIsColliding false))

(event Input|KeyboardEvents|Add
  (params (Key :type Key%20Structure :default "None"))
  ;[0.9577 0.3385 1] Simple Update Life System +
  (:Pressed
    (CallFunction|UpdateLife 1 false)))

(event Input|KeyboardEvents|Subtract
  (params (Key :type Key%20Structure :default "None"))
  ;[1 0.4851 0.2522] Simple Update Life System -
  (:Pressed
    (CallFunction|UpdateLife -1 false)))

(event Input|KeyboardEvents|K
  (params (Key :type Key%20Structure :default "None"))
  ;[0.519 1 0.9602] Simple Respawn Mechanic
  (:Pressed
    (Actor|DestroyActor)))

(fn ConstructionScript)

(fn SetInputMapping
  (bind _asplayer_controller (Utilities|Casting|CastToPlayerController (Pawn|GetController)))
  (Utilities|IsValid (PlayerController|LocalPlayerSubsystems|GetEnhancedInputLocalPlayerSubsystem _asplayer_controller)
    (:Is%20Valid
      (Input|AddMappingContext (PlayerController|LocalPlayerSubsystems|GetEnhancedInputLocalPlayerSubsystem _asplayer_controller) "/Game/Input/IMC_Character.IMC_Character" 0 "(bIgnoreAllPressedKeysUntilRelease=True,bForceImmediately=False,bNotifyUserSettings=False)"))))

(fn UpdateLife
  (params (Amount :type Integer) (Max%20Life :type Boolean))
  (if Max%20Life
    (if (> (Variables|Default|GetMaxLife) 3)
      (Variables|Default|SetMaxLife (+ (Variables|Default|GetMaxLife) Amount))
      (Default|RefreshHorizontalBox (Variables|Default|GetHudLifeRef))
      (elif (and (== (Variables|Default|GetMaxLife) 3) (> Amount 0))
        (Variables|Default|SetMaxLife (+ (Variables|Default|GetMaxLife) Amount))
        (Default|RefreshHorizontalBox (Variables|Default|GetHudLifeRef))))
    (else
      (Variables|Default|SetLife (+ (Variables|Default|GetLife) Amount))
      (Default|RefreshHorizontalBox (Variables|Default|GetHudLifeRef))
      (Utilities|FlowControl|Sequence
        (:then_0
          (if (< (Variables|Default|GetLife) 0)
            (CallFunction|DeathSystem)))
        (:then_1
          (if (> (Variables|Default|GetLife) (Variables|Default|GetMaxLife))
            (Variables|Default|SetLife (Variables|Default|GetMaxLife))))))))

(fn DeathSystem
  (Physics|SetSimulatePhysics (Variables|Character|GetMesh) true)
  (Variables|/Script/Engine.PlayerController|SetbShowMouseCursor (Game|GetPlayerController 0) true)
  (bind _returnvalue (UserInterface|CreateWidget "/Game/HUD/WBP_GameOver.WBP_GameOver_C"))
  (UserInterface|Viewport|AddtoViewport _returnvalue 0))

(fn PauseMenu
  (bind _returnvalue (Game|GetPlayerController 0))
  (if (not (Variables|Default|GetisPauseMenuOpened))
    (Variables|Default|SetisPauseMenuOpened true)
    (bind _returnvalue_2 (UserInterface|CreateWidget "/Game/HUD/WBP_PauseMenu.WBP_PauseMenu_C" _returnvalue))
    (bind _output_get (Variables|Default|SetPauseMenuWidget _returnvalue_2))
    (UserInterface|Viewport|AddtoViewport _output_get 0)
    (Input|SetInputModeUIOnly _returnvalue (Variables|Default|GetPauseMenuWidget) "DoNotLock" false)
    (Variables|/Script/Engine.PlayerController|SetbShowMouseCursor (Game|GetPlayerController 0) true)
    (Game|SetGamePaused true)
    (else
      (Variables|Default|SetisPauseMenuOpened false)
      (Widget|RemovefromParent (Variables|Default|GetPauseMenuWidget))
      (Game|SetGamePaused false)
      (Input|SetInputModeGameOnly _returnvalue false)
      (Variables|/Script/Engine.PlayerController|SetbShowMouseCursor (Game|GetPlayerController 0) true))))

(fn OnSlap
  (if (Variables|Default|GetIsColliding)
    (Variables|Default|SetIsAttacking true)
    (Development|SetHiddeninGame (Variables|Default|GetHitbox) true false)
    (Development|PrintString "Slap Attack")
    (Default|GetDamage (Variables|Default|GetCurrentEnemy) (Math|Float|Truncate (Variables|Default|GetDamage)))))