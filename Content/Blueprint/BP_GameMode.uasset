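; BP_GameMode is a game mode Blueprint that respawns the player after the BP_Player character is destroyed.
; On BeginPlay it binds to the player character's OnDestroyed event.
; When that fires, it waits briefly, spawns a new BP_Player at the SpawnTransform variable and has the first player controller possess it.
; It then calls Respawn to rebind the event on the new pawn, so the cycle repeats.
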(event Custom|OnDestroyed_
  (params (DestroyedActor :type Actor%20Object%20Reference))
  (Utilities|FlowControl|Delay 2.0)
  (bind _returnvalue (Game|SpawnActorfromClass "/Game/Blueprint/Player/BP_Player.BP_Player_C" (Variables|Default|GetSpawnTransform) "AdjustIfPossibleButAlwaysSpawn" "MultiplyWithRoot" 0 0))
  (Pawn|Possess (Game|GetPlayerController 0) _returnvalue)
  (CallFunction|Respawn))

(event Custom|Respawn
  (bind _asbp_player (Utilities|Casting|CastToBP_Player (Game|GetPlayerCharacter 0)))
  (Game|BindEventtoOnDestroyed _asbp_player (delegate Custom|OnDestroyed_)))

(event EventBeginPlay
  (bind _asbp_player (Utilities|Casting|CastToBP_Player (Game|GetPlayerCharacter 0)))
  (Game|BindEventtoOnDestroyed _asbp_player (delegate Custom|OnDestroyed_)))

(fn ConstructionScript)