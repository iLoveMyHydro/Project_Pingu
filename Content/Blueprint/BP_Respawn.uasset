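; BP_Respawn is a checkpoint trigger that records a spawn point when the player touches it.
; On BeginPlay it registers itself as the Respawn reference in the BP_GameManager game instance.
; When BP_Player overlaps its box, it copies the player's current transform, rather than its own, into BP_GameMode's SpawnTransform, then sets and debug-prints a SpawnpointSet flag.
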(event OnComponentBeginOverlap(Box)
  (params (OverlappedComponent :type Primitive%20Component%20Object%20Reference) (OtherActor :type Actor%20Object%20Reference) (OtherComp :type Primitive%20Component%20Object%20Reference) (OtherBodyIndex :type Integer) (bFromSweep :type Boolean) (SweepResult :type Hit%20Result%20Structure%20%28by%20ref%29))
  (bind _asbp_player (Utilities|Casting|CastToBP_Player OtherActor))
  (bind _asbp_game_mode (Utilities|Casting|CastToBP_GameMode (Game|GetGameMode)))
  (Variables|/Game/Blueprint/BP_GameMode.BP_GameMode_C|SetSpawnTransform _asbp_game_mode (Transformation|GetActorTransform _asbp_player))
  (bind _output_get (Variables|Default|SetSpawnpointSet true))
  (Development|PrintString (Utilities|String|ToString(Boolean) _output_get)))

(event EventBeginPlay
  (bind _asbp_game_manager (Utilities|Casting|CastToBP_GameManager (Game|GetGameInstance)))
  (Variables|/Game/Blueprint/BP_GameManager.BP_GameManager_C|Setrespawn _asbp_game_manager self))

(fn ConstructionScript)